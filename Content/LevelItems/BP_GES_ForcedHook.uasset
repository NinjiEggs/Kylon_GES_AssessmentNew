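; Forced hook level item that pulls the third-person player character to its own position and then removes itself.
; Each tick it runs a large sphere trace around its Sphere component and casts the hit actor to the player character.
; On a hit it teleports the character to the sphere's location in one step, as the VInterpTo has identical current and target, then destroys itself.
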(event Collision|EventActorBeginOverlap
  (params (OtherActor :type Actor%20Object%20Reference)))

(event EventTick
  (params (DeltaSeconds :type Float%20%28single-precision%29))
  (bind _sphere (Variables|Default|GetSphere))
  (bind _returnvalue (Transformation|GetWorldLocation _sphere))
  (bind _outhit (Collision|SphereTraceByChannel _returnvalue _returnvalue 2e+03 "TraceTypeQuery6" false 0 "None" true "(R=1.000000,G=0.000000,B=0.000000,A=1.000000)" "(R=0.000000,G=1.000000,B=0.000000,A=1.000000)" 1.0))
  (bind _asbp_third_person_character (Utilities|Casting|CastToBP_ThirdPersonCharacter (.HitActor (Collision|BreakHitResult _outhit))))
  (bind _output_get (Variables|Default|SetPlayer%20Reference _asbp_third_person_character))
  (Transformation|SetWorldLocation (Variables|/Script/Engine.Actor|GetRootComponent _output_get) (Math|Interpolation|VInterpTo (Transformation|GetWorldLocation (Variables|Default|GetSphere)) _returnvalue DeltaSeconds 5e+01) false true)
  (Actor|DestroyActor))

(fn ConstructionScript)