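; Large enemy that turns to face the player and fires large stone balls when it sees them.
; PawnSensing sightings of BP_ThirdPersonCharacter snap the actor's rotation toward the pawn, then a one-second Delay paces the shots.
; Each shot spawns BP_StoneBall_Large at ProjectileSpawn and launches its sphere forward with a mass-independent velocity-change impulse.
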(event OnSeePawn(PawnSensing)
  (params (Pawn :type Pawn%20Object%20Reference))
  (bind _returnvalue (Transformation|GetActorLocation Pawn))
  (bind _projectilespawn (Variables|Default|GetProjectileSpawn))
  ;[0.06771 0.06771 0.06771] Shoot at Player In Range
  (Utilities|Casting|CastToBP_ThirdPersonCharacter Pawn)
  (Transformation|SetActorRotation (Math|Rotator|FindLookatRotation (Transformation|GetActorLocation) (Math|Vector|MakeVector (.x _returnvalue) (.y _returnvalue) (.z _returnvalue))))
  (Utilities|FlowControl|Delay 1.0)
  (bind _returnvalue_2 (Game|SpawnActorfromClass "/Game/LevelItems/BP_StoneBall_Large.BP_StoneBall_Large_C" (Transformation|GetWorldTransform _projectilespawn) "Undefined" "MultiplyWithRoot" 0 0))
  (Physics|AddImpulse (Variables|/Game/LevelItems/BP_StoneBall_Large.BP_StoneBall_Large_C|GetSphere _returnvalue_2) (* (Math|Vector|GetForwardVector _projectilespawn) 2e+04) "None" true))

(event EventBeginPlay)

(event Collision|EventActorBeginOverlap
  (params (OtherActor :type Actor%20Object%20Reference)))

(event EventTick
  (params (DeltaSeconds :type Float%20%28single-precision%29)))

(fn ConstructionScript)