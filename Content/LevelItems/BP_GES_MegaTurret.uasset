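; BP_GES_MegaTurret is a turret that turns toward a player it sees through PawnSensing and fires projectiles at them.
; After a short delay it spawns a BP_GES_SpawnBall at ProjectileSpawn and launches its four spheres forward with a large velocity-change impulse.
; A boss cooldown event bound on the player character sets a flag that inserts a longer pause before the next shot.
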(event OnSeePawn(PawnSensing)
  (params (Pawn :type Pawn%20Object%20Reference))
  (bind _returnvalue (Transformation|GetActorLocation Pawn))
  (bind _projectilespawn (Variables|Default|GetProjectileSpawn))
  ;[0.06771 0.06771 0.06771] Shoot at Player In Range
  (if (Variables|Default|GetCooldown%20Active?)
    (Utilities|FlowControl|Delay 2.0)
    (Variables|Default|SetCooldown%20Active? false))
  (Utilities|Casting|CastToBP_ThirdPersonCharacter Pawn)
  (Transformation|SetActorRotation (Math|Rotator|FindLookatRotation (Transformation|GetActorLocation) (Math|Vector|MakeVector (.x _returnvalue) (.y _returnvalue) (.z _returnvalue))))
  (Utilities|FlowControl|Delay 0.53)
  (bind _returnvalue_2 (Game|SpawnActorfromClass "/Game/LevelItems/BP_GES_SpawnBall.BP_GES_SpawnBall_C" (Transformation|GetWorldTransform _projectilespawn) "Undefined" "MultiplyWithRoot" 0 0))
  (Physics|AddImpulse (Variables|/Game/LevelItems/BP_GES_SpawnBall.BP_GES_SpawnBall_C|GetSphere _returnvalue_2) (* (Math|Vector|GetForwardVector _projectilespawn) 5.3e+05) "None" true))

(event Custom|Cooldown
  (Variables|Default|SetCooldown%20Active? true))

(event EventBeginPlay
  (bind _asbp_third_person_character (Utilities|Casting|CastToBP_ThirdPersonCharacter (Game|GetPlayerCharacter 0)))
  (EventDispatchers|BindEventtoCreateBossCooldown _asbp_third_person_character (delegate Custom|Cooldown)))

(event Collision|EventActorBeginOverlap
  (params (OtherActor :type Actor%20Object%20Reference)))

(event EventTick
  (params (DeltaSeconds :type Float%20%28single-precision%29)))

(fn ConstructionScript)