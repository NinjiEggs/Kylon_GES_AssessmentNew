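; BP_GES_GraviHook_Massive is a large-radius gravity hook level item that pulls the player toward its sphere on right-click.
; Each Tick, a 7500-unit sphere trace checks for BP_ThirdPersonCharacter, stores the reference, binds its OnMouseRightPressed event and sets IsInRange.
; When that event fires in range, VInterpTo steps the player's root from the supplied last location toward the sphere, without sweeping.
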(event Custom|Check%20if%20Player%20in%20Radius
  (params (Last%20Player%20Location :type Vector))
  (if (Variables|Default|GetIs%20In%20Range?)
    (Transformation|SetWorldLocation (Variables|/Script/Engine.Actor|GetRootComponent (Variables|Default|GetPlayer%20Reference)) (Math|Interpolation|VInterpTo Last%20Player%20Location (Transformation|GetWorldLocation (Variables|Default|GetSphere)) (stale EventTick DeltaSeconds) 5e+01) false false)))

(event Collision|EventActorBeginOverlap
  (params (OtherActor :type Actor%20Object%20Reference)))

(event EventTick
  (params (DeltaSeconds :type Float%20%28single-precision%29))
  (bind _sphere (Variables|Default|GetSphere))
  (bind _returnvalue (Transformation|GetWorldLocation _sphere))
  (bind _outhit (Collision|SphereTraceByChannel _returnvalue _returnvalue 7.5e+03 "TraceTypeQuery4" false 0 "None" true "(R=1.000000,G=0.000000,B=0.000000,A=1.000000)" "(R=0.000000,G=1.000000,B=0.000000,A=1.000000)" 1.0))
  (bind _asbp_third_person_character (Utilities|Casting|CastToBP_ThirdPersonCharacter (.HitActor (Collision|BreakHitResult _outhit)))
    (:then
      (bind _output_get (Variables|Default|SetPlayer%20Reference _asbp_third_person_character))
      (EventDispatchers|BindEventtoOnMouseRightPressed _output_get (delegate Custom|Check%20if%20Player%20in%20Radius))
      (Variables|Default|SetIs%20In%20Range? true))
    (:CastFailed
      (Variables|Default|SetIs%20In%20Range? false))))

(fn ConstructionScript)