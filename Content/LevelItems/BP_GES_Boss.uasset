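; BP_GES_Boss is a boss level item with a cat mesh that turns to face the player when it sees them.
; Pawn sensing filters for the third-person character, then snaps the actor's rotation toward it; despite a shooting comment, no firing logic is present.
; A Delay on Tick throttles a flag toggle that alternates the cat's second material slot between a morph-demo and an anisotropic material, roughly every 0.6 seconds.
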(event OnSeePawn(PawnSensing)
  (params (Pawn :type Pawn%20Object%20Reference))
  (bind _returnvalue (Transformation|GetActorLocation Pawn))
  ;[0.06771 0.06771 0.06771] Shoot at Player In Range
  (Utilities|Casting|CastToBP_ThirdPersonCharacter Pawn)
  (Transformation|SetActorRotation (Math|Rotator|FindLookatRotation (Transformation|GetActorLocation) (Math|Vector|MakeVector (.x _returnvalue) (.y _returnvalue) (.z _returnvalue)))))

(event EventBeginPlay)

(event Collision|EventActorBeginOverlap
  (params (OtherActor :type Actor%20Object%20Reference)))

(event EventTick
  (params (DeltaSeconds :type Float%20%28single-precision%29))
  (bind _cat (Variables|Default|Getcat))
  (Utilities|FlowControl|Delay 0.6)
  (if (Variables|Default|GetTex1?)
    (Rendering|Material|SetMaterial _cat 1 "/Engine/Functions/Engine_MaterialFunctions02/ExampleContent/TextureBasedWPO/TextureBasedMorphDemo.TextureBasedMorphDemo")
    (Variables|Default|SetTex1? false)
    (else
      (Rendering|Material|SetMaterial _cat 1 "/Game/Assets/anisotropic1.anisotropic1")
      (Variables|Default|SetTex1? true))))

(fn ConstructionScript)