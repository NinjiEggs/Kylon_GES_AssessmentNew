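; GameInstance Blueprint that holds game-completion and per-level progress flags for three levels and persists them to disk.
; On Init it loads the save slot if one exists, casts it to BP_GES_SaveGame and copies its flags into the instance.
; SaveGame creates a fresh save object, copies the current flags into it and writes it to the same single slot.
; A ReturnCurrentSkin function is present but empty.
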(event Custom|SaveGame
  (bind _returnvalue (SaveGame|CreateSaveGameObject "/Game/Instance/BP_GES_SaveGame.BP_GES_SaveGame_C"))
  (Variables|/Game/Instance/BP_GES_SaveGame.BP_GES_SaveGame_C|SetSaveBeatenGame? _returnvalue (Variables|Default|GetBeatenGame?))
  (Variables|/Game/Instance/BP_GES_SaveGame.BP_GES_SaveGame_C|SetSaveBeatLevel1? _returnvalue (Variables|Default|GetBeatLevel1?))
  (Variables|/Game/Instance/BP_GES_SaveGame.BP_GES_SaveGame_C|SetSaveBeatLevel2? _returnvalue (Variables|Default|GetBeatLevel2?))
  (Variables|/Game/Instance/BP_GES_SaveGame.BP_GES_SaveGame_C|SetSaveBeatLevel3? _returnvalue (Variables|Default|GetBeatLevel3?))
  (SaveGame|SaveGametoSlot _returnvalue "Slot1"))

(event Custom|LoadGame
  (bind _returnvalue (SaveGame|DoesSaveGameExist "Slot1"))
  (if _returnvalue
    (bind _returnvalue_2 (SaveGame|LoadGamefromSlot "Slot1"))
    (bind _asbp_ges_save_game (Utilities|Casting|CastToBP_GES_SaveGame _returnvalue_2))
    (Variables|Default|SetBeatenGame? (Variables|/Game/Instance/BP_GES_SaveGame.BP_GES_SaveGame_C|GetSaveBeatenGame? _asbp_ges_save_game))
    (Variables|Default|SetBeatLevel1? (Variables|/Game/Instance/BP_GES_SaveGame.BP_GES_SaveGame_C|GetSaveBeatLevel1? _asbp_ges_save_game))
    (Variables|Default|SetBeatLevel2? (Variables|/Game/Instance/BP_GES_SaveGame.BP_GES_SaveGame_C|GetSaveBeatLevel2? _asbp_ges_save_game))
    (Variables|Default|SetBeatLevel3? (Variables|/Game/Instance/BP_GES_SaveGame.BP_GES_SaveGame_C|GetSaveBeatLevel3? _asbp_ges_save_game))))

(event EventInit
  (CallFunction|LoadGame))

(fn ReturnCurrentSkin)